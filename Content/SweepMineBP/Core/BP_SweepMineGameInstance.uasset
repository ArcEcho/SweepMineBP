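; Game instance for a Minesweeper game that owns the game flow, minefield and win check.
; A state machine macro swaps start menu, HUD, game over and victory widgets.
; Starting a game sizes the grid by difficulty, randomly picks mine cells, spawns BP_MineContainer actors and tallies eight-way neighbor counts.
; Revealing recursively flood-fills empty cells in four directions, counting down safe cells to victory, while mark toggles update the HUD's mine count.
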(event Custom|OnMineContainerToggleMarked
  (params (IsMarked :type Boolean))
  (if IsMarked
    (bind _output_get (Variables|Default|SetPredictedRemainingMineCount (- (Variables|Default|GetPredictedRemainingMineCount) 1)))
    (Default|OnUpdateRemainingMineCount (Variables|Default|GetHUDWidget) _output_get)
    (else
      (bind _output_get_2 (Variables|Default|SetPredictedRemainingMineCount (+ (Variables|Default|GetPredictedRemainingMineCount) 1)))
      (Default|OnUpdateRemainingMineCount (Variables|Default|GetHUDWidget) _output_get_2))))

(event Custom|ShowMainMenu
  (bind _returnvalue (Game|GetPlayerController 0))
  (Utilities|TransittoState "NewEnumerator0"
    (:Succeed
      (Utilities|IsValid (Variables|Default|GetStartMenuWidget)
        (:Is%20Valid
          _)
        (:Is%20Not%20Valid
          (bind _returnvalue_2 (UserInterface|CreateWidget "/Game/SweepMineBP/UI/S_Menu.S_Menu_C" _returnvalue))
          (Variables|Default|SetStartMenuWidget _returnvalue_2)))
      (Input|SetInputModeUIOnly _returnvalue (Variables|Default|GetStartMenuWidget) "DoNotLock")
      (UserInterface|Viewport|AddtoViewport (Variables|Default|GetStartMenuWidget) 0))))

(event Custom|ShowGameOverUI
  (bind _returnvalue (Game|GetPlayerController 0))
  (Utilities|TransittoState "NewEnumerator2"
    (:Succeed
      (CallFunction|NotifyGameOverEvent)
      (Utilities|IsValid (Variables|Default|GetGameOverWidget)
        (:Is%20Valid
          _)
        (:Is%20Not%20Valid
          (bind _returnvalue_2 (UserInterface|CreateWidget "/Game/SweepMineBP/UI/S_GameOver.S_GameOver_C" _returnvalue))
          (Variables|Default|SetGameOverWidget _returnvalue_2)))
      (Input|SetInputModeUIOnly _returnvalue (Variables|Default|GetGameOverWidget) "DoNotLock")
      (UserInterface|Viewport|AddtoViewport (Variables|Default|GetGameOverWidget) 0))))

(event Custom|NotifyGameOverEvent
  (CallFunction|ReleaseContainerRef)
  (Default|CallGameOver))

(event Custom|ShowGameVictoryUI
  (bind _returnvalue (Game|GetPlayerController 0))
  (Utilities|TransittoState "NewEnumerator3"
    (:Succeed
      (CallFunction|NotifyGameOverEvent)
      (Utilities|IsValid (Variables|Default|GetGameVictoryWidget)
        (:Is%20Valid
          _)
        (:Is%20Not%20Valid
          (bind _returnvalue_2 (UserInterface|CreateWidget "/Game/SweepMineBP/UI/S_GameVictory.S_GameVictory_C" _returnvalue))
          (Variables|Default|SetGameVictoryWidget _returnvalue_2)))
      (Input|SetInputModeUIOnly _returnvalue (Variables|Default|GetGameVictoryWidget) "DoNotLock")
      (UserInterface|Viewport|AddtoViewport (Variables|Default|GetGameVictoryWidget) 0))))

(event Custom|StartGame
  (bind _returnvalue (Game|GetPlayerController 0))
  (CallFunction|InitializeFieldParamsbyDifficulty)
  (CallFunction|CreateLevel)
  (Utilities|TransittoState "NewEnumerator1"
    (:Succeed
      (Utilities|IsValid (Variables|Default|GetHUDWidget)
        (:Is%20Valid
          _)
        (:Is%20Not%20Valid
          (bind _returnvalue_2 (UserInterface|CreateWidget "/Game/SweepMineBP/UI/S_HUD.S_HUD_C" _returnvalue))
          (Variables|Default|SetHUDWidget _returnvalue_2)))
      (Input|SetInputModeGameandUI _returnvalue 0 "DoNotLock" false)
      (UserInterface|Viewport|AddtoViewport (Variables|Default|GetHUDWidget) 0)
      (Default|OnUpdateRemainingMineCount (Variables|Default|GetHUDWidget) (Variables|Default|GetPredictedRemainingMineCount)))))

(fn DistributeMines
  (bind _candicateindexarray (LocalVariables|GetCandicateIndexArray))
  (bind _returnvalue (Utilities|Array|Length _candicateindexarray))
  (bind _returnvalue_2 (- _returnvalue 1))
  (bind _returnvalue_3 (Math|Random|RandomIntegerinRange 0 _returnvalue_2))
  (for _index (range 0 (- (Variables|Default|GetComlumCount) 1))
    (for _index_2 (range 0 (- (Variables|Default|GetRowCount) 1))
      (bind _outindex (CallFunction|GetIndexfromColumnandRow _index _index_2))
      (Utilities|Array|SetArrayElem (LocalVariables|GetCandicateIndexArray) _outindex _outindex true)))
  (for _index_3 (range 1 (Variables|Default|GetMineCount))
    (Utilities|Set|Add (LocalVariables|GetResultSet) (Utilities|Array|Get(acopy) _candicateindexarray _returnvalue_3))
    (Utilities|Array|RemoveIndex (LocalVariables|GetCandicateIndexArray) _returnvalue_3))
  (return (LocalVariables|GetResultSet)))

(fn CreateMineField
  ;[1 1 1] Spawn Mines
  (for _index (range 0 (- (Variables|Default|GetComlumCount) 1))
    (for _index_2 (range 0 (- (Variables|Default|GetRowCount) 1))
      (bind _returnvalue (Game|SpawnActorfromClass "/Game/SweepMineBP/Blueprints/BP_MineContainer.BP_MineContainer_C" (Math|Transform|MakeTransform (Math|Vector|MakeVector (- (* _index (Variables|Default|GetMineContainerSpacing)) (/ (* (- (Variables|Default|GetRowCount) 1) (Variables|Default|GetMineContainerSpacing)) 2.0)) (- (* _index_2 (Variables|Default|GetMineContainerSpacing)) (/ (* (- (Variables|Default|GetRowCount) 1) (Variables|Default|GetMineContainerSpacing)) 2.0)) 5e+01)) "Undefined" 0 (Utilities|Set|Contains (Variables|Default|GetDistributeResult) (+ _index_2 (* _index (Variables|Default|GetRowCount)))) _index _index_2))
      (bind _outindex (CallFunction|GetIndexfromColumnandRow _index _index_2))
      (Utilities|Array|SetArrayElem (Variables|Default|GetMineContainerArray) _outindex _returnvalue true)))
  ;[1 1 1] Statistic neighbor mine count
  (for _index_3 (range 0 (- (Variables|Default|GetComlumCount) 1))
    (for _index_4 (range 0 (- (Variables|Default|GetRowCount) 1))
      (bind _outindex_2 (CallFunction|GetIndexfromColumnandRow _index_3 _index_4))
      (if (Variables|/Game/SweepMineBP/Blueprints/BP_MineContainer.BP_MineContainer_C|GetHasMine (Utilities|Array|Get(acopy) (Variables|Default|GetMineContainerArray) _outindex_2))
        (CallFunction|AddNeghborContainerNeighborMineCount _index_3 _index_4)))))

(fn InitializeFieldParamsbyDifficulty
  (switch int (Variables|Default|GetDifficulty)
    (:0
      (Variables|Default|SetMineCount 5)
      (Variables|Default|SetRowCount 5)
      (Variables|Default|SetComlumCount 5))
    (:1
      (Variables|Default|SetMineCount 20)
      (Variables|Default|SetRowCount 10)
      (Variables|Default|SetComlumCount 10)))
  (Variables|Default|SetRemainingEmptyContainerCount (- (* (Variables|Default|GetRowCount) (Variables|Default|GetComlumCount)) (Variables|Default|GetMineCount)))
  (Variables|Default|SetPredictedRemainingMineCount (Variables|Default|GetMineCount)))

(fn AdjustCameraPosition)

(fn GetIndexfromColumnandRow
  (params (InColumnIndex :type Integer) (InRowIndex :type Integer))
  (return (+ (* InColumnIndex (Variables|Default|GetRowCount)) InRowIndex)))

(fn AddNeghborContainerNeighborMineCount
  (params (InColumnIndex :type Integer) (InRowIndex :type Integer))
  (bind _returnvalue (- InRowIndex 1))
  (bind _returnvalue_2 (+ InRowIndex 1))
  ;[1 1 1] Top Left
  (CallFunction|TryAddNeighborMineCount (- InColumnIndex 1) _returnvalue_2)
  ;[1 1 1] Top
  (CallFunction|TryAddNeighborMineCount InColumnIndex _returnvalue_2)
  ;[1 1 1] Top Right
  (CallFunction|TryAddNeighborMineCount (+ InColumnIndex 1) _returnvalue_2)
  ;[1 1 1] Left
  (CallFunction|TryAddNeighborMineCount (- InColumnIndex 1) InRowIndex)
  ;[1 1 1] Right
  (CallFunction|TryAddNeighborMineCount (+ InColumnIndex 1) InRowIndex)
  ;[1 1 1] Bottom Left
  (CallFunction|TryAddNeighborMineCount (- InColumnIndex 1) _returnvalue)
  ;[1 1 1] Bottom
  (CallFunction|TryAddNeighborMineCount InColumnIndex _returnvalue)
  ;[1 1 1] Bottom Right
  (CallFunction|TryAddNeighborMineCount (+ InColumnIndex 1) _returnvalue))

(fn TryAddNeighborMineCount
  (params (InColumnIndex :type Integer) (InRowIndex :type Integer))
  (Utilities|IsOutOfRange InColumnIndex InRowIndex
    (:false
      (bind _outindex (CallFunction|GetIndexfromColumnandRow InColumnIndex InRowIndex))
      (Variables|/Game/SweepMineBP/Blueprints/BP_MineContainer.BP_MineContainer_C|SetNeighborMineCount (Utilities|Array|Get(acopy) (Variables|Default|GetMineContainerArray) _outindex) (+ (Variables|/Game/SweepMineBP/Blueprints/BP_MineContainer.BP_MineContainer_C|GetNeighborMineCount (Utilities|Array|Get(acopy) (Variables|Default|GetMineContainerArray) _outindex)) 1)))))

(fn TryDetectNeighborContainer
  (params (InColumnIndex :type Integer) (InRowIndex :type Integer))
  ;[1 1 1] Determin whether to detect neigbor container
  (bind _targetminecontainer (CallFunction|GetMineContainer InColumnIndex InRowIndex))
  (Utilities|IsValid _targetminecontainer
    (:Is%20Valid
      (if (not (Math|Boolean|ORBoolean (Variables|/Game/SweepMineBP/Blueprints/BP_MineContainer.BP_MineContainer_C|GetHasBeenChecked _targetminecontainer) (Variables|/Game/SweepMineBP/Blueprints/BP_MineContainer.BP_MineContainer_C|GetHasBeenMarked _targetminecontainer) (Variables|/Game/SweepMineBP/Blueprints/BP_MineContainer.BP_MineContainer_C|GetHasMine _targetminecontainer)))
        (Default|ShowNeighborMineCount _targetminecontainer)
        ;[1 1 1] Check victory when any container is checked
        (bind _result (CallFunction|CheckVictory))
        (if _result
          (CallFunction|ShowGameVictoryUI)
          (elif (== (Variables|/Game/SweepMineBP/Blueprints/BP_MineContainer.BP_MineContainer_C|GetNeighborMineCount _targetminecontainer) 0)
            ;[1 1 1] Top
            (CallFunction|TryDetectNeighborContainer InColumnIndex (+ InRowIndex 1))
            ;[1 1 1] Left
            (CallFunction|TryDetectNeighborContainer (- InColumnIndex 1) InRowIndex)
            ;[1 1 1] Right
            (CallFunction|TryDetectNeighborContainer (+ InColumnIndex 1) InRowIndex)
            ;[1 1 1] Bottom
            (CallFunction|TryDetectNeighborContainer InColumnIndex (- InRowIndex 1))))))))

(fn GetMineContainer
  (params (InColumnIndex :type Integer) (InRowIndex :type Integer))
  (Utilities|IsOutOfRange InColumnIndex InRowIndex
    (:true
      (return 0))
    (:false
      (bind _outindex (CallFunction|GetIndexfromColumnandRow InColumnIndex InRowIndex))
      (return (Utilities|Array|Get(acopy) (Variables|Default|GetMineContainerArray) _outindex)))))

(fn CreateLevel
  (bind _outresultset (CallFunction|DistributeMines))
  (Variables|Default|SetDistributeResult _outresultset)
  (CallFunction|CreateMineField)
  (Default|CallMineFieldCreatingCompleted)
  (CallFunction|AdjustCameraPosition))

(fn ReleaseContainerRef
  (Utilities|Array|Clear (Variables|Default|GetMineContainerArray)))

(fn SetDifficulty
  (params (InDifficulty :type Integer))
  (Variables|Default|SetDifficulty InDifficulty))

(fn CheckVictory
  (bind _output_get (Variables|Default|SetRemainingEmptyContainerCount (- (Variables|Default|GetRemainingEmptyContainerCount) 1)))
  (return (== _output_get 0)))