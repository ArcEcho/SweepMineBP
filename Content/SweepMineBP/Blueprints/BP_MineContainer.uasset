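; Minesweeper cell actor that holds a mine or neighbor count and reacts to being checked or marked.
; Checking either explodes with radial force and shows game over, or asks the game instance to detect neighbors by row and column.
; Marking toggles a reused flag actor, capped by the game instance's predicted remaining mines.
; Revealed cells get a material and color-mapped count text; all cells self-destroy shortly after game over.
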(event Custom|OnGameOver
  ;[1 1 1] When game is over, destroy this actor after 0.5s for explode effect
  (Utilities|FlowControl|Delay 0.5)
  (Actor|DestroyActor))

(event Custom|OnChecked
  (bind _returnvalue (Transformation|GetActorLocation))
  (if (Variables|Default|GetHasMine)
    (Default|ShowGameOverUI (Variables|Default|GetGameInstanceRef))
    ;[1 1 1] If it  has mine, just explodes.
    (Actor|DestroyActor)
    (Game|SpawnActorfromClass "/Game/SweepMineBP/Blueprints/BP_MineExplodeRadialForce.BP_MineExplodeRadialForce_C" (Math|Conversions|ToTransform(Vector) _returnvalue) "AlwaysSpawn" 0 0)
    (Effects|SpawnEmitteratLocation "/Game/SweepMineBP/Particles/P_Explosion.P_Explosion" _returnvalue)
    (Audio|PlaySound2D "/Game/SweepMineBP/Audio/Explosion_Cue.Explosion_Cue")
    (else
      ;[1 1 1] Try to detect neigbor mine container
      (Default|TryDetectNeighborContainer (Variables|Default|GetGameInstanceRef) (Variables|Default|GetColumnIndex) (Variables|Default|GetRowIndex))
      (Audio|PlaySound2D "/Game/SweepMineBP/Audio/Blueprints_TextPop01.Blueprints_TextPop01"))))

(event Custom|OnMarked
  (if (Variables|Default|GetHasBeenChecked)
    (Audio|PlaySound2D "/Game/SweepMineBP/Audio/Blueprints_TextPop03.Blueprints_TextPop03")
    (elif (Variables|Default|GetHasBeenMarked)
      (Rendering|SetActorHiddenInGame (Variables|Default|GetMarkedFlag) true)
      (Variables|Default|SetHasBeenMarked false)
      (Default|OnMineContainerToggleMarked (Variables|Default|GetGameInstanceRef) (Variables|Default|GetHasBeenMarked) :!label _label)
      (if (Variables|Default|GetHasBeenMarked)
        (Audio|PlaySound2D "/Game/SweepMineBP/Audio/Building_Attachment_Stereo.Building_Attachment_Stereo")
        (else
          (Audio|PlaySound2D "/Game/SweepMineBP/Audio/Gold_Dissapear05_Stereo.Gold_Dissapear05_Stereo")))
      (else
        ;[1 1 1] When max marked, do nothing
        (if (== (Variables|/Game/SweepMineBP/Core/BP_SweepMineGameInstance.BP_SweepMineGameInstance_C|GetPredictedRemainingMineCount (Variables|Default|GetGameInstanceRef)) 0)
          (Audio|PlaySound2D "/Game/SweepMineBP/Audio/Blueprints_TextPop03.Blueprints_TextPop03")
          (else
            (Utilities|IsValid (Variables|Default|GetMarkedFlag)
              (:Is%20Valid
                (Rendering|SetActorHiddenInGame (Variables|Default|GetMarkedFlag) false))
              (:Is%20Not%20Valid
                (bind _returnvalue (Game|SpawnActorfromClass "/Game/SweepMineBP/Blueprints/BP_Flag.BP_Flag_C" (Math|Transform|MakeTransform (+ (Transformation|GetActorLocation) "0,0.000000,60.000000") "0, 0, 0" "0.500000,0.500000,0.500000") "Undefined" 0 0))
                (Variables|Default|SetMarkedFlag _returnvalue)))
            (Variables|Default|SetHasBeenMarked true)
            (goto _label)))))))

(event EventBeginPlay
  (bind _asbp_sweep_mine_game_instance (Utilities|Casting|CastToBP_SweepMineGameInstance (Game|GetGameInstance)))
  (bind _output_get (Variables|Default|SetGameInstanceRef _asbp_sweep_mine_game_instance))
  (EventDispatchers|BindEventtoGameOver _output_get (delegate Custom|OnGameOver)))

(event Collision|EventActorBeginOverlap
  (params (OtherActor :type Actor%20Object%20Reference)))

(fn ConstructionScript)

(fn SetChecked)

(fn ShowNeighborMineCount
  (bind _neighborminecount (Variables|Default|GetNeighborMineCount))
  (bind _neighborminecounttext (Variables|Default|GetNeighborMineCountText))
  (Variables|Default|SetHasBeenChecked true)
  (if (== _neighborminecount 0)
    ;[1 1 1] No mine around
    (Rendering|Material|SetMaterial (Variables|Default|GetMineContainerCube) 0 "/Game/SweepMineBP/Materials/MInst_MineContainer_NoMine.MInst_MineContainer_NoMine")
    (else
      ;[1 1 1] Has mine around
      (Rendering|Components|TextRender|SetText _neighborminecounttext (Utilities|Text|ToText(Integer) _neighborminecount))
      (Rendering|Components|TextRender|SetTextRenderColor (Variables|Default|GetNeighborMineCountText) (Math|Conversions|ToColor(LinearColor) (.Value (Utilities|Map|Find (Variables|Default|GetCountToColorMap) (Variables|Default|GetNeighborMineCount)))))
      (Rendering|SetVisibility _neighborminecounttext true false)
      (Rendering|Material|SetMaterial (Variables|Default|GetMineContainerCube) 0 "/Game/SweepMineBP/Materials/MInst_MineContainer_HasMineInNeighborbiourhood.MInst_MineContainer_HasMineInNeighborbiourhood"))))