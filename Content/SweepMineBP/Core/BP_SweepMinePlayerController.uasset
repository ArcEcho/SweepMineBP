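; Player controller for the Minesweeper game that turns mouse clicks into actions on mine tiles under the cursor.
; Each button press does a complex cursor trace and casts the hit actor to BP_MineContainer.
; Left click calls OnChecked and right click calls OnMarked, with a DoOnce per button that resets on release so each press fires once.
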(event EventBeginPlay)

(event EventTick
  (params (DeltaSeconds :type Float%20%28single-precision%29)))

(event Input|ActionEvents|InputActionLMB
  (params (Key :type Key%20Structure :default "AnyKey"))
  (:Pressed
    (Utilities|FlowControl|DoOnce false :!label _label
      (:Completed
        (bind _asbp_mine_container (Utilities|Casting|CastToBP_MineContainer (.HitActor (Collision|BreakHitResult (.HitResult (Game|Player|GetHitResultUnderCursorbyChannel "TraceTypeQuery3" true))))))
        (Default|OnChecked _asbp_mine_container))))
  (:Released
    (goto _label Reset)))

(event Input|ActionEvents|InputActionRMB
  (params (Key :type Key%20Structure :default "AnyKey"))
  (:Pressed
    (Utilities|FlowControl|DoOnce false :!label _label
      (:Completed
        (bind _asbp_mine_container (Utilities|Casting|CastToBP_MineContainer (.HitActor (Collision|BreakHitResult (.HitResult (Game|Player|GetHitResultUnderCursorbyChannel "TraceTypeQuery3" true))))))
        (Default|OnMarked _asbp_mine_container))))
  (:Released
    (goto _label Reset)))

(fn ConstructionScript)